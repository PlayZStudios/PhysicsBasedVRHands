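; VR hand actor that visualises tracked hand joints; only the left hand runs, as the right-hand path is disconnected.
; Each Tick clears the markers, reads the 26 hand-tracking keypoints and redraws them as small static mesh instances.
; The same transforms pose a PoseableMesh bone by bone in world space, composed with a rotation correction offset.
; The left Manny XR physics asset is reassigned inside that per-joint loop.
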(event `self.ReceiveTick`
  (params (DeltaSeconds :type "Float (single-precision)"))
  (`self.ClearHand`)
  (bind _transforms (`self.Get Joint Transforms` "Left"))
  (`self.DrawHand` _transforms))

(fn `ClearHand`
  (`InstancedStaticMeshComponent.ClearInstances` (`self.InstancedStaticMesh`)))

(fn `DrawHand`
  (params (Transforms :type "Array of Transform Structure"))
  (locals (`Poseable mesh` :type "PoseableMeshComponent Object Reference") (LeftBones :type "Array of String"))
  (for (_array_element _array_index) Transforms
    (`InstancedStaticMeshComponent.AddInstance` (`self.InstancedStaticMesh`) _array_element true)
    (bind (_location _rotation) (`self.GetHandMeshBoneLocationRotation` (.location _array_element) (`KismetMathLibrary.Conv_RotatorToQuaternion` (.rotation _array_element))))
    (`PoseableMeshComponent.SetBoneTransformByName` (`self.PoseableMesh`) (`KismetStringLibrary.Conv_StringToName` (`|GetArrayItem` (`local.LeftBones`) _array_index)) (`KismetMathLibrary.MakeTransform` _location (`KismetMathLibrary.Quat_Rotator` _rotation)) "WorldSpace")
    (`SkinnedMeshComponent.SetPhysicsAsset` (`self.PoseableMesh`) "/Game/XRMannequins/Meshes/SKM_MannyXR_left_Physics.SKM_MannyXR_left_Physics" false)))

(fn `Get Joint Transforms`
  (params (Hand :type "EControllerHand Enum" :default "Left"))
  (returns (Transforms :type "Array of Transform Structure"))
  (locals (`Joint Transforms` :type "Array of Transform Structure"))
  (bind _handtrackingstate (`HeadMountedDisplayFunctionLibrary.GetHandTrackingState` null "UnrealWorldSpace" Hand))
  (bind (_bvalid _devicename _applicationinstanceid _xrspacetype _hand _trackingstatus _handkeylocations _handkeyrotations) (break `XRHandTrackingState` _handtrackingstate))
  (if _bvalid
    (if (and (== (`KismetArrayLibrary.Array_Length` _handkeylocations) 26) (== (`KismetArrayLibrary.Array_Length` _handkeyrotations) 26))
      (for (_array_element _array_index) _handkeylocations
        (`KismetArrayLibrary.Array_Add` (`local.Joint Transforms`) (`KismetMathLibrary.MakeTransform` _array_element (`KismetMathLibrary.Quat_Rotator` (`|GetArrayItem` _handkeyrotations _array_index)) (0.01 0.01 0.01))))
      (return (`local.Joint Transforms`))
      (else
        (return (`local.Joint Transforms`))))))

(fn `GetHandMeshBoneLocationRotation`
  (params (handKeyLocation :type "Vector Structure") (handKeyRotation :type "Quat Structure"))
  (returns (Location :type "Vector Structure") (Rotation :type "Quat Structure"))
  (bind (_returnvalue_location _returnvalue_rotation) (`KismetMathLibrary.BreakTransform` (`KismetMathLibrary.ComposeTransforms` (`KismetMathLibrary.MakeTransform` (0.0 0.0 0.0) (`self.BoneCorrectionOffset`)) (`KismetMathLibrary.MakeTransform` handKeyLocation (`KismetMathLibrary.Quat_Rotator` handKeyRotation)))))
  (return _returnvalue_location (`KismetMathLibrary.Conv_RotatorToQuaternion` _returnvalue_rotation)))

(fn `UserConstructionScript`)